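; TurtleTwo is a turtle actor that emerges from a ring gate, travels toward a given Destination actor, then exits with a hyperjump and destroys itself.
; SetDestination chains timelines: the ring grows and spins, the turtle appears, and the spin reverses before the gate hides.
; Movement repeats in bursts, with a brief material swap and pause between them, until an overlap with Destination triggers the jump's scaling, movement and sound.
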(event `Set Destination`
  (params (Destination :type "/Game/Blueprints/Destination Object Reference"))
  (bind _ring (`self.Ring`))
  ;[1 1 1] Расширение врат из которой появится черепаха
  (bind (_direction _resize) (`Timeline|Circle_Resize` :!via `PlayFromStart`)
    (:`Update`
      (`SceneComponent.SetRelativeScale3D` (`self.Ring`) _resize))
    (:`Finished`
      ;[1 1 1] Сначала происходит нарастающее вращение врат, затем появление черепахи.
      ; После этого прекращается вращение и исчезают врата.
      (bind (_direction_2 _rotate) (`Timeline|Circle_Rotate` :!via `PlayFromStart` :!label _label)
        (:`Update`
          (`SceneComponent.K2_AddWorldRotation` (`self.Ring`) (`KismetMathLibrary.MakeRotator` 0.0 _rotate) false false))
        (:`Finished`
          (if (`self.FirstRotationDone`)
            (`SceneComponent.SetVisibility` _ring false false)
            (`SceneComponent.K2_SetWorldRotation` _ring (struct :`Pitch` 90.0) false false)
            ;[1 1 1] Движение вперед
            (bind (_direction_3 _x_move) (`Timeline|Move` :!via `PlayFromStart` :!label _label_2)
              (:`Update`
                (`self.K2_AddActorWorldOffset` _x_move))
              (:`Finished`
                ;[1 1 1] Проверка на достижение черепахой цели
                (if (`self.IsOverlappingActor` Destination)
                  ;[1 1 1] Финиширование черепахи с последующим эффектом "гиперпрыжка"
                  (bind (_direction_4 _jumpdrivesizing _jumdriveactivatemove) (`Timeline|JumpDrive` :!via `PlayFromStart`)
                    (:`Update`
                      (`SceneComponent.SetRelativeScale3D` (`self.Cylinder`) _jumpdrivesizing)
                      (`self.K2_AddActorWorldOffset` _jumdriveactivatemove))
                    (:`Finished`
                      (`self.K2_DestroyActor`))
                    (:`JumpDriveActivate`
                      (`GameplayStatics.PlaySoundAtLocation` "/Game/Audio/TurtleTwoSpawnSound.TurtleTwoSpawnSound" (`self.K2_GetActorLocation`) (struct) 1.0 1.0 1.0 null null null)))
                  (else
                    ;[1 1 1] Остановка и смена цвета черепашки
                    (`PrimitiveComponent.SetMaterial` (`self.Cylinder`) 0 "/Game/Materials/Button_material.Button_material")
                    (`KismetSystemLibrary.Delay` 0.5)
                    (`PrimitiveComponent.SetMaterial` (`self.Cylinder`) 0 "/Game/Materials/TurtleTwoMaterial.TurtleTwoMaterial")
                    (goto _label_2 :!via `PlayFromStart`)))))
            (else
              (`GameplayStatics.PlaySoundAtLocation` "/Game/Audio/TurtleTwoSpawnSound.TurtleTwoSpawnSound" (`self.K2_GetActorLocation`) (struct) 1.0 1.0 1.0 null null null)
              (`SceneComponent.SetVisibility` (`self.Cylinder`) true false)
              (set `self.FirstRotationDone` true)
              (goto _label :!via `ReverseFromEnd`))))
        (:`Rotate Sound`
          (`GameplayStatics.PlaySoundAtLocation` "/Game/Audio/RotatingSound.RotatingSound" (`self.K2_GetActorLocation`) (struct) 1.0 1.0 0.0 null null null))))))

(fn `UserConstructionScript`)