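; Nest is a spawner Blueprint that releases a turtle when its ActivateNest event is called.
; The event switches on IdNest to choose one of three classes: Turtle, TurtleTwo or TurtleThree.
; Each turtle spawns at the Sphere component's world transform and receives the nest's Destination through SetDestination.
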(event `Activate Nest`
  (bind _destination (`self.Destination`))
  (bind _returnvalue (`SceneComponent.K2_GetComponentToWorld` (`self.Sphere`)))
  (switch `int` (`self.Id_Nest`)
    (:`1`
      (bind _returnvalue_2 (`|SpawnActorFromClass` "/Game/Blueprints/Turtle.Turtle_C" _returnvalue "Undefined" "OverrideRootScale" null null))
      (`/Game/Blueprints/Turtle.Set Destination` _returnvalue_2 _destination))
    (:`2`
      (bind _returnvalue_3 (`|SpawnActorFromClass` "/Game/Blueprints/TurtleTwo.TurtleTwo_C" _returnvalue "Undefined" "OverrideRootScale" null null))
      (`/Game/Blueprints/TurtleTwo.Set Destination` _returnvalue_3 _destination))
    (:`3`
      (bind _returnvalue_4 (`|SpawnActorFromClass` "/Game/Blueprints/TurtleThree.TurtleThree_C" _returnvalue "Undefined" "OverrideRootScale" null null))
      (`/Game/Blueprints/TurtleThree.Set Destination` _returnvalue_4 _destination))))

(fn `UserConstructionScript`)