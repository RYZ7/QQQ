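; Turtle actor that travels toward a given destination actor, animated by scaling its sphere component, then destroys itself.
; SetDestination plays a wind sound and inflates the sphere via the Resize timeline, then a looping Move timeline squashes it while applying world offsets without sweep.
; After each Move cycle it checks overlap with the destination, either replaying wind and moving again or playing an end sound, deflating via Unsize and destroying the actor.
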(event `Set Destination`
  (params (Destination :type "/Game/Blueprints/Destination Object Reference"))
  (`GameplayStatics.PlaySoundAtLocation` "/Game/Audio/wind.wind" (`self.K2_GetActorLocation`) (struct) 1.0 1.0 0.0 null null null)
  ;[1 1 1] При появлении черепаха надувается
  (bind (_direction _resize) (`Timeline|Resize` :!via `PlayFromStart`)
    (:`Update`
      (`SceneComponent.SetRelativeScale3D` (`self.Sphere`) _resize))
    (:`Finished`
      ;[1 1 1] Непрерывное передвижение черепахи с эффектом "скукоживания"
      (bind (_direction_2 _x_move _sizing) (`Timeline|Move` :!via `PlayFromStart` :!label _label)
        (:`Update`
          (`SceneComponent.SetRelativeScale3D` (`self.Sphere`) _sizing)
          (`self.K2_AddActorWorldOffset` _x_move))
        (:`Finished`
          (if (`self.IsOverlappingActor` Destination)
            ;[1 1 1] Финиш черепахи с эффектом сдувания и звуком
            (`GameplayStatics.PlaySoundAtLocation` "/Game/Audio/TurtleOneEnd.TurtleOneEnd" (`self.K2_GetActorLocation`) (struct) 1.0 1.0 0.0 null null null)
            (bind (_direction_3 _unsize) (`Timeline|Unsize` :!via `PlayFromStart`)
              (:`Update`
                (`SceneComponent.SetRelativeScale3D` (`self.Sphere`) _unsize))
              (:`Finished`
                (`self.K2_DestroyActor`)))
            (else
              ;[1 1 1] Звук при передвижении
              (`GameplayStatics.PlaySoundAtLocation` "/Game/Audio/wind.wind" (`self.K2_GetActorLocation`) (struct) 1.0 1.0 0.0 null null null)
              (goto _label :!via `PlayFromStart`))))))))

(fn `UserConstructionScript`)