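; TurtleThreeEgg is an egg actor that may hatch a TurtleThree.
; On SpawnEgg it plays a spawn sound and grows its Sphere through the EggGrowth timeline.
; When growth finishes, a coin flip either destroys the egg or, after a random delay, spawns a turtle at the egg's transform, passes it the Destination, and then destroys the egg.
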(event `SpawnEgg`
  (params (Destination :type "/Game/Blueprints/Destination Object Reference"))
  (`GameplayStatics.PlaySoundAtLocation` "/Game/Audio/Turtle3SpawnEggSound.Turtle3SpawnEggSound" (`self.K2_GetActorLocation`) (struct) 1.0 1.0 0.5 null null null)
  ;[1 1 1] Рост яйца
  (bind (_direction _eggsize) (`Timeline|EggGrowth` :!via `PlayFromStart`)
    (:`Update`
      (`SceneComponent.SetRelativeScale3D` (`self.Sphere`) _eggsize))
    (:`Finished`
      ;[1 1 1] 50 на 50 того, что вылупится черепаха
      (if (`KismetMathLibrary.RandomBool`)
        ;[1 1 1] Вылупление черепахи
        (`KismetSystemLibrary.Delay` (`KismetMathLibrary.RandomFloatInRange` 0.0 15.0))
        (bind _returnvalue (`|SpawnActorFromClass` "/Game/Blueprints/TurtleThree.TurtleThree_C" (`self.GetTransform`) "Undefined" "OverrideRootScale" null null))
        (`/Game/Blueprints/TurtleThree.Set Destination` _returnvalue Destination)
        (`self.K2_DestroyActor`)
        (else
          (`self.K2_DestroyActor`))))))

(fn `UserConstructionScript`)