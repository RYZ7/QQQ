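; TurtleThree is a turtle actor that hatches from an egg and works its way toward a Destination actor passed to SetDestination.
; Chained timelines drive it: Birth cracks the egg sphere, then Move advances and grows the turtle.
; Without a Destination overlap, Reverse backs it up under a swapped material, randomly spawns a TurtleThreeEgg with the same Destination, then restarts Move.
; On overlap, Dying spins and lifts it before destruction.
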(event `Set Destination`
  (params (Destination :type "/Game/Blueprints/Destination Object Reference"))
  (bind _returnvalue (`self.K2_GetActorLocation`))
  ;[1 1 1] Анимация яйца и рождение черепахи из неё
  (bind (_direction _eggcrack) (`Timeline|Birth` :!via `PlayFromStart`)
    (:`Update`
      (`SceneComponent.SetRelativeScale3D` (`self.Sphere`) _eggcrack))
    (:`Finished`
      (`GameplayStatics.PlaySoundAtLocation` "/Game/Audio/TurtleThreeSpawnSound.TurtleThreeSpawnSound" _returnvalue (struct) 1.0 1.0 0.0 null null null)
      (`SceneComponent.SetVisibility` (`self.Sphere`) false false)
      ;[1 1 1] Движение вперед и увеличение размеров черепахи
      (bind (_direction_2 _movement_x _scaling) (`Timeline|Move` :!via `PlayFromStart` :!label _label)
        (:`Update`
          (`self.K2_AddActorLocalOffset` _movement_x)
          (bind _output_get (set `self.Scale` (+ (`SceneComponent.K2_GetComponentScale` (`self.Cube`)) _scaling)))
          (`SceneComponent.SetRelativeScale3D` (`self.Cube`) _output_get))
        (:`Finished`
          (if (`self.IsOverlappingActor` Destination)
            ;[1 1 1] Финиш черепахи
            (bind (_direction_3 _rotate _ascend) (`Timeline|Dying`)
              (:`Update`
                (`self.K2_AddActorWorldRotation` (`KismetMathLibrary.MakeRotator` 0.0 0.0 _rotate))
                (`self.K2_AddActorWorldOffset` _ascend))
              (:`Finished`
                (`self.K2_DestroyActor`)))
            (else
              ;[1 1 1] Движение назад
              ; Черепаха откладывает яйцо при 50/50 шансах, из которой потом вылупится еще черепаха.
              (`PrimitiveComponent.SetMaterial` (`self.Cube`) 0 "/Game/Materials/Button_material.Button_material")
              (bind (_direction_4 _movement_x_2) (`Timeline|Reverse` :!via `PlayFromStart`)
                (:`Update`
                  (`self.K2_AddActorLocalOffset` _movement_x_2))
                (:`Finished`
                  (if (`KismetMathLibrary.RandomBool`)
                    (bind _returnvalue_2 (`|SpawnActorFromClass` "/Game/Blueprints/TurtleThreeEgg.TurtleThreeEgg_C" (`self.GetTransform`) "Undefined" "OverrideRootScale" null null))
                    (`/Game/Blueprints/TurtleThreeEgg.SpawnEgg` _returnvalue_2 Destination))
                  (`PrimitiveComponent.SetMaterial` (`self.Cube`) 0 "/Game/Materials/TurtleMaterial.TurtleMaterial")
                  (goto _label :!via `PlayFromStart`))))))))
    (:`EggCrackSound`
      (`GameplayStatics.PlaySoundAtLocation` "/Game/Audio/PressSound1.PressSound1" _returnvalue (struct) 1.0 1.0 0.0 null null null))))

(fn `UserConstructionScript`)