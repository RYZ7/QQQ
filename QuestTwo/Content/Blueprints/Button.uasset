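; Interactive button that triggers a nest activation when the player presses Interact while inside its trigger box.
; Overlap with a DefaultPawn opens or closes a Gate that filters the Interact input, with input enabled for player controller 0 at BeginPlay.
; The ButtonAnimation macro plays a sound, then lerps the button transform down and back with two timelines.
; Once the button returns to rest, it calls ActivateNest on the Nest.
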(event `self.ReceiveBeginPlay`
  (bind (_returnvalue_location _returnvalue_rotation _returnvalue_scale) (`KismetMathLibrary.BreakTransform` (`SceneComponent.GetRelativeTransform` (`self.Button`))))
  ;[1 1 1] Инициализация
  (set `self.NonPressedPosition` (`KismetMathLibrary.MakeTransform` _returnvalue_location _returnvalue_rotation _returnvalue_scale))
  (set `self.PressPosition` (`KismetMathLibrary.MakeTransform` (- _returnvalue_location (0.0 0.0 30.0))))
  (`self.EnableInput` (`GameplayStatics.GetPlayerController` 0)))

(event `InputAction|Interact` :consume false
  (params (Key :type "Key Structure"))
  ;[1 1 1] Триггер на действие
  (:`Pressed`
    (`/Engine/EditorBlueprintResources/StandardMacros.Gate` true :!label _label
      (:`Exit`
        (`GameplayStatics.PlaySoundAtLocation` "/Game/Audio/PressSound1.PressSound1" (`self.K2_GetActorLocation`) (struct) 1.0 1.0 0.0 null null null)
        (bind (_direction _buttonpress) (`Timeline|ButtonPress` :!via `PlayFromStart`)
          (:`Update`
            (`SceneComponent.K2_SetRelativeTransform` (`self.Button`) (`KismetMathLibrary.TLerp` (`self.NonPressedPosition`) (`self.PressPosition`) _buttonpress) false false))
          (:`Finished`
            (bind (_direction_2 _buttonpress_2) (`Timeline|ButtonUnPress` :!via `ReverseFromEnd`)
              (:`Update`
                (`SceneComponent.K2_SetRelativeTransform` (`self.Button`) (`KismetMathLibrary.TLerp` (`self.NonPressedPosition`) (`self.PressPosition`) _buttonpress_2) false false))
              (:`Finished`
                ;[1 1 1] Активация гнезда
                (`/Game/Blueprints/Nest.Activate Nest` (`self.Nest`))))))))))

(event `self.Box.OnComponentBeginOverlap`
  (params (OverlappedComponent :type "PrimitiveComponent Object Reference") (OtherActor :type "Actor Object Reference") (OtherComp :type "PrimitiveComponent Object Reference") (OtherBodyIndex :type Integer) (bFromSweep :type Boolean) (SweepResult :type "HitResult Structure (by ref)"))
  ;[1 1 1] Триггер на действие
  (cast `DefaultPawn` OtherActor)
  (goto _label :!via `Open`))

(event `self.Box.OnComponentEndOverlap`
  (params (OverlappedComponent :type "PrimitiveComponent Object Reference") (OtherActor :type "Actor Object Reference") (OtherComp :type "PrimitiveComponent Object Reference") (OtherBodyIndex :type Integer))
  ;[1 1 1] Триггер на действие
  (cast `DefaultPawn` OtherActor)
  (goto _label :!via `Close`))

(fn `UserConstructionScript`)